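; Health pickup actor that restores the MySteve character's health when touched.
; On capsule overlap with MySteve, a DoOnce gate lets it call HealthUpdate if Health is below 100, then the pickup destroys itself.
; Every Tick it also looks up MySteve with GetActorOfClass and destroys itself if that Health is above 99, even without being touched.
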(event `self.ReceiveTick`
  (params (DeltaSeconds :type "Float (single-precision)"))
  (bind _returnvalue (`GameplayStatics.GetActorOfClass` "/Game/Characters/MySteve.MySteve_C"))
  (`/Engine/EditorBlueprintResources/StandardMacros.IsValid` _returnvalue
    (:`Is Valid`
      (if (> (`Steve.Health` _returnvalue) 99.0)
        (`self.K2_DestroyActor`)))))

(event `self.Capsule.OnComponentBeginOverlap`
  (params (OverlappedComponent :type "PrimitiveComponent Object Reference") (OtherActor :type "Actor Object Reference") (OtherComp :type "PrimitiveComponent Object Reference") (OtherBodyIndex :type Integer) (bFromSweep :type Boolean) (SweepResult :type "HitResult Structure (by ref)"))
  (bind _asmy_steve (cast `/Game/Characters/MySteve` OtherActor))
  (`/Engine/EditorBlueprintResources/StandardMacros.IsValid` _asmy_steve
    (:`Is Valid`
      (`/Engine/EditorBlueprintResources/StandardMacros.DoOnce` false
        (:`Completed`
          (if (< (`Steve.Health` _asmy_steve) 100.0)
            (`Steve.HealthUpdate` _asmy_steve))
          (`self.K2_DestroyActor`))))))

(fn `UserConstructionScript`)